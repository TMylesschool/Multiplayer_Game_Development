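; BP_AutoDoor is an automatic door that swings open when something overlaps its box trigger and closes after the trigger empties.
; BeginPlay caches the closed rotation and derives the open rotation by adding a yaw offset.
; The TL_Door timeline lerps the door mesh between the two rotations, playing on overlap and reversing after a delay if no actors remain.
; An IsOpen flag guards both transitions, which also print debug strings.
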(event OnComponentBeginOverlap(BoxCollision)
  (params (OverlappedComponent :type Primitive%20Component%20Object%20Reference) (OtherActor :type Actor%20Object%20Reference) (OtherComp :type Primitive%20Component%20Object%20Reference) (OtherBodyIndex :type Integer) (bFromSweep :type Boolean) (SweepResult :type Hit%20Result%20Structure%20%28by%20ref%29))
  (if (not (Variables|Default|GetIsOpen))
    (Variables|Default|SetIsOpen true)
    (Development|PrintString "Hello")
    (Development|PrintString (Utilities|String|ToString(Rotator) (Variables|Default|GetOpenRot)))
    (bind _newtrack_0 (Timeline|TL_Door Play)
      (:Update
        (Transformation|SetRelativeRotation (Variables|Default|GetDoorMesh) (Math|Rotator|Lerp(Rotator) (Variables|Default|GetClosedRot) (Variables|Default|GetOpenRot) _newtrack_0) false false)))))

(event OnComponentEndOverlap(BoxCollision)
  (params (OverlappedComponent :type Primitive%20Component%20Object%20Reference) (OtherActor :type Actor%20Object%20Reference) (OtherComp :type Primitive%20Component%20Object%20Reference) (OtherBodyIndex :type Integer))
  (Utilities|FlowControl|Delay (Variables|Default|GetCloseDelay))
  (if (Variables|Default|GetIsOpen)
    (if (== (Utilities|Array|Length (Collision|GetOverlappingActors (Variables|Default|GetBoxCollision) 0 :!class /Script/Engine.PrimitiveComponent)) 0)
      (Variables|Default|SetIsOpen false)
      (Development|PrintString "Hello")
      (Development|PrintString (Utilities|String|ToString(Rotator) (Variables|Default|GetClosedRot)))
      (bind _newtrack_0 (Timeline|TL_Door Reverse)
        (:Update
          (Transformation|SetRelativeRotation (Variables|Default|GetDoorMesh) (Math|Rotator|Lerp(Rotator) (Variables|Default|GetClosedRot) (Variables|Default|GetOpenRot) _newtrack_0) false false))))))

(event EventBeginPlay
  (Variables|Default|SetIsOpen false)
  (Variables|Components|SetOpenAngle 9e+01)
  (Variables|Default|SetClosedRot (Variables|/Script/Engine.SceneComponent|GetRelativeRotation (Variables|Default|GetDoorMesh)))
  (Variables|Default|SetOpenRot (Math|Rotator|CombineRotators (Variables|Default|GetClosedRot) (Math|Rotator|MakeRotator 0.0 0.0 (Variables|Components|GetOpenAngle))))
  (Variables|Default|SetOpenSpeed 1.5)
  (Variables|Default|SetCloseDelay 1.0))

(event Collision|EventActorBeginOverlap
  (params (OtherActor :type Actor%20Object%20Reference)))

(event EventTick
  (params (DeltaSeconds :type Float%20%28single-precision%29)))

(fn ConstructionScript)